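; BP_Stalagtite is a falling-rock hazard Blueprint that supplies the sound feedback for each stage of the fall.
; Three events for rock triggered, falling and hit swap the sound on a single AudioComponent to a warning, whoosh or rockfall cue and play it.
; The graph holds no trigger or movement logic, and the construction script is empty.
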(event `self.BPOnRockHit`
  (bind _audiocomponent (`self.AudioComponent`))
  (`AudioComponent.SetSound` _audiocomponent "/Game/Audio/SC_RockFall.SC_RockFall")
  (`AudioComponent.Play` _audiocomponent 0.0))

(event `self.OnRockTriggered`
  (bind _audiocomponent (`self.AudioComponent`))
  (`AudioComponent.SetSound` _audiocomponent "/Game/Audio/SC_FallingWarning.SC_FallingWarning")
  (`AudioComponent.Play` _audiocomponent 0.0))

(event `self.OnRockFalling`
  (bind _audiocomponent (`self.AudioComponent`))
  (`AudioComponent.SetSound` _audiocomponent "/Game/Audio/SC_Woosh.SC_Woosh")
  (`AudioComponent.Play` _audiocomponent 0.0))

(fn `UserConstructionScript`)